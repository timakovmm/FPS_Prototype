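; Weapon manager component for BP_Main_Character that holds the carried weapons and handles firing, switching and ammo pickup.
; New weapons spawn only if that class isn't already owned, start with a full clip and are equipped immediately.
; Scrolling wraps through the list, moving weapons between sockets and hiding inactive ones.
; Equipping also sets walk speed, updates HUD name and ammo, and signals whether a rifle is equipped.
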(fn StartFire
  (Utilities|IsValid (Variables|Weapon|GetEquippedWeapon)
    (:Is%20Valid
      (Default|StartFire (Variables|Weapon|GetEquippedWeapon)))))

(fn StopFire
  (Utilities|IsValid (Variables|Weapon|GetEquippedWeapon)
    (:Is%20Valid
      (Default|StopFire (Variables|Weapon|GetEquippedWeapon)))))

(fn CreateWeapon
  (params (WeaponType :type BP%20Main%20Weapon%20Class%20Reference))
  (bind _cancreateweapon_ (Weapon|GetCanCreateWeapon WeaponType))
  (if _cancreateweapon_
    (bind _returnvalue (Game|SpawnActorfromClass WeaponType (Math|Transform|MakeTransform "0, 0, 0") "AlwaysSpawn" 0 0))
    (bind _output_get (LocalVariables|SetNewCurrentWeapon _returnvalue))
    (bind _returnvalue_2 (Utilities|Array|Add (Variables|Weapon|GetRefWeapon) _output_get))
    (Variables|Weapon|SetWeaponIndex _returnvalue_2)
    (Default|ChangeCurrentAmmo (LocalVariables|GetNewCurrentWeapon) (.MaxClipAmmo (Utilities|Struct|BreakStruct_Ammo (Variables|/Game/Blueprints/Weapons/BP_Main_Weapon.BP_Main_Weapon_C|GetAmmoData (LocalVariables|GetNewCurrentWeapon)))))
    (Weapon|UnEquipWeapon)
    (bind _success_ (Weapon|EquipWeapon))
    (return _success_)
    (else
      (return false))))

(fn AddNewWeapon
  (params (WeaponType :type BP%20Main%20Weapon%20Class%20Reference))
  (bind _success_ (Weapon|CreateWeapon WeaponType))
  (return _success_))

(fn EquipWeapon
  (if (Utilities|Array|IsValidIndex (Variables|Weapon|GetRefWeapon) (Variables|Weapon|GetWeaponIndex))
    (bind _asbp_main_character (Utilities|Casting|CastToBP_Main_Character (Components|GetOwner)))
    (bind _output_get (Variables|Weapon|SetEquippedWeapon (Utilities|Array|Get(acopy) (Variables|Weapon|GetRefWeapon) (Variables|Weapon|GetWeaponIndex))))
    (Transformation|AttachComponentToComponent _output_get (Variables|/Game/Blueprints/Characters/BP_Main_Character.BP_Main_Character_C|GetSkeletalMesh _asbp_main_character) (Variables|Weapon|GetEqSocketWeapon) "KeepRelative" "KeepRelative" "KeepRelative" true)
    (Rendering|SetActorHiddenInGame (Variables|Weapon|GetEquippedWeapon) false)
    (Variables|/Game/Blueprints/Weapons/BP_Main_Weapon.BP_Main_Weapon_C|SetIsEquipped? (Variables|Weapon|GetEquippedWeapon) true)
    (bind _asbp_main_character_2 (Utilities|Casting|CastToBP_Main_Character (Components|GetOwner)))
    (if (Variables|/Game/Blueprints/Characters/BP_Main_Character.BP_Main_Character_C|GetIsRunning? _asbp_main_character_2)
      (Variables|/Script/Engine.CharacterMovementComponent|SetMaxWalkSpeed (Variables|/Script/Engine.Character|GetCharacterMovement _asbp_main_character_2) (+ (Variables|/Game/Blueprints/Weapons/BP_Main_Weapon.BP_Main_Weapon_C|GetMaxWalkSpeed (Variables|Weapon|GetEquippedWeapon)) (Variables|/Game/Blueprints/Characters/BP_Main_Character.BP_Main_Character_C|GetRunSpeed _asbp_main_character_2)))
      (else
        (Variables|/Script/Engine.CharacterMovementComponent|SetMaxWalkSpeed (Variables|/Script/Engine.Character|GetCharacterMovement _asbp_main_character_2) (Variables|/Game/Blueprints/Weapons/BP_Main_Weapon.BP_Main_Weapon_C|GetMaxWalkSpeed (Variables|Weapon|GetEquippedWeapon)))))
    (bind _currentui (Class|BPIUserInterface|BPIGetCurrentUI(Message) (HUD|GetHUD (Game|GetPlayerController 0))))
    (Class|BPIUserInterface|BPIGetWeaponName(Message) _currentui (Variables|/Game/Blueprints/Weapons/BP_Main_Weapon.BP_Main_Weapon_C|GetWeaponName (Variables|Weapon|GetEquippedWeapon)))
    (Default|ChangeCurrentAmmo (Variables|Weapon|GetEquippedWeapon) (Variables|/Game/Blueprints/Weapons/BP_Main_Weapon.BP_Main_Weapon_C|GetCurrentAmmo (Variables|Weapon|GetEquippedWeapon)))
    (Default|ChangeLeftAmmo (Variables|Weapon|GetEquippedWeapon) (Variables|/Game/Blueprints/Weapons/BP_Main_Weapon.BP_Main_Weapon_C|GetLeftAmmo (Variables|Weapon|GetEquippedWeapon)))
    (Default|CallNewEquippedWeapon true (Utilities|Select :Index (Variables|/Game/Blueprints/Weapons/BP_Main_Weapon.BP_Main_Weapon_C|GetAmmoType (Variables|Weapon|GetEquippedWeapon)) :NewEnumerator0 true :NewEnumerator1 false))
    (return true)
    (else
      (return false))))

(fn UnEquipWeapon
  (Utilities|IsValid (Variables|Weapon|GetEquippedWeapon)
    (:Is%20Valid
      (bind _asbp_main_character (Utilities|Casting|CastToBP_Main_Character (Components|GetOwner)))
      (Transformation|AttachComponentToComponent (Variables|Weapon|GetEquippedWeapon) (Variables|/Game/Blueprints/Characters/BP_Main_Character.BP_Main_Character_C|GetSkeletalMesh _asbp_main_character) (Variables|Weapon|GetUnEqSocketWeapon) "KeepRelative" "KeepRelative" "KeepRelative" true)
      (Rendering|SetActorHiddenInGame (Variables|Weapon|GetEquippedWeapon) true)
      (Variables|/Game/Blueprints/Weapons/BP_Main_Weapon.BP_Main_Weapon_C|SetIsEquipped? (Variables|Weapon|GetEquippedWeapon) false))))

(fn GetCanCreateWeapon
  (params (WeaponType :type BP%20Main%20Weapon%20Class%20Reference))
  (if (Utilities|Array|IsValidIndex (Variables|Weapon|GetRefWeapon))
    (for _array_element (Variables|Weapon|GetRefWeapon)
      (if (== WeaponType (Utilities|GetClass _array_element))
        (LocalVariables|SetFoundWeapon? true)))
    (return (not (LocalVariables|GetFoundWeapon?)))
    (else
      (return true))))

(fn ScrollWeapon
  (params (ScrollUp :type Boolean))
  (if ScrollUp
    (if (> (+ (Variables|Weapon|GetWeaponIndex) 1) (Utilities|Array|LastIndex (Variables|Weapon|GetRefWeapon)))
      (Variables|Weapon|SetWeaponIndex 0)
      (else
        (Variables|Weapon|SetWeaponIndex (+ (Variables|Weapon|GetWeaponIndex) 1))))
    (elif (< (- (Variables|Weapon|GetWeaponIndex) 1) 0)
      (Variables|Weapon|SetWeaponIndex (Utilities|Array|LastIndex (Variables|Weapon|GetRefWeapon)))
      (else
        (Variables|Weapon|SetWeaponIndex (- (Variables|Weapon|GetWeaponIndex) 1)))))
  (Weapon|UnEquipWeapon)
  (Weapon|EquipWeapon))

(fn AddAmmobyWeapon
  (params (AddAmmo :type Integer) (AmmoType :type E_AmmoType%20Enum :default "NewEnumerator0"))
  (if (Utilities|Array|IsValidIndex (Variables|Weapon|GetRefWeapon))
    (for _array_element (Variables|Weapon|GetRefWeapon)
      (if (and (Utilities|Enum|Equal(Enum) AmmoType (Default|GetAmmoType _array_element)) (< (Variables|/Game/Blueprints/Weapons/BP_Main_Weapon.BP_Main_Weapon_C|GetLeftAmmo _array_element) (.MaxAmmo (Utilities|Struct|BreakStruct_Ammo (Variables|/Game/Blueprints/Weapons/BP_Main_Weapon.BP_Main_Weapon_C|GetAmmoData _array_element)))))
        (Default|AddAmmo _array_element AddAmmo)
        (return true)))))