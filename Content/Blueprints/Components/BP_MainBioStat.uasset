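; Component that manages a generic bio stat, filled to its maximum on BeginPlay and reduced by damage.
; All changes pass through ChangeStat, which clamps between zero and MaxStat and stops regeneration when full.
; Damage lowers the stat, halts regeneration and sets a one-shot delay timer.
; Regeneration runs on a looping timer whose stored handle allows cancellation, with RegenerateStat adding RegenerationPower per step.
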(event EventBeginPlay
  (Stat|ChangeStat (Variables|Stat|GetMaxStat)))

(fn AddStat
  (params (AddStat :type Float%20%28single-precision%29))
  (if (< (Variables|Stat|GetCurrentStat) (Variables|Stat|GetMaxStat))
    (Stat|ChangeStat (+ (Variables|Stat|GetCurrentStat) AddStat))
    (return true)))

(fn DecreaseStat
  (params (DamageValue :type Float%20%28single-precision%29))
  (Utilities|Time|SetTimerbyEvent (EventDispatchers|CreateEvent :!event StartRegenerateStat) (Variables|Stat|GetStartRegenerationDelay))
  (Stat|ChangeStat (- (Variables|Stat|GetCurrentStat) DamageValue))
  (Stat|StopRegenerateStat))

(fn ChangeStat
  (params (NewStat :type Float%20%28single-precision%29))
  (if (!= NewStat (Variables|Stat|GetCurrentStat))
    (Variables|Stat|SetCurrentStat (Math|Float|Clamp(Float) NewStat 0.0 (Variables|Stat|GetMaxStat)))
    (if (== (Variables|Stat|GetCurrentStat) (Variables|Stat|GetMaxStat))
      (Stat|StopRegenerateStat))))

(fn RegenerateStat
  (Stat|ChangeStat (+ (Variables|Stat|GetCurrentStat) (Variables|Stat|GetRegenerationPower))))

(fn StartRegenerateStat
  (bind _returnvalue (Utilities|Time|SetTimerbyEvent (EventDispatchers|CreateEvent :!event RegenerateStat) (Variables|Stat|GetRegenerationRate) true))
  (Variables|Stat|SetRegenerationHandleTimer _returnvalue))

(fn StopRegenerateStat
  (if (Utilities|Time|IsValidTimerHandle (Variables|Stat|GetRegenerationHandleTimer))
    (Utilities|Time|ClearandInvalidateTimerbyHandle (Variables|Stat|GetRegenerationHandleTimer))))

(fn TakeDamage
  (params (DamageValue :type Float%20%28single-precision%29))
  (Stat|DecreaseStat DamageValue))