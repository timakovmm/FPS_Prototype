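; Boss health stat component that reports the boss's health to the HUD and ends the game when it runs out.
; ChangeStat runs the parent logic, then passes CurrentStat to the boss health message through the HUD's UI interface.
; At zero or below, it calls MakeDeath on its owner, cast to SteelPlayerCharacter, then its own MakeDeath calls FinishGame on BP_Main_GameMode.
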(event EventBeginPlay
  (|CallParentFunction) ; This node is disabled and will not be called.\nDrag off pins to build functionality.
)

(event EventTick
  (params (DeltaSeconds :type Float%20%28single-precision%29)))

(fn ChangeStat
  (params (NewStat :type Float%20%28single-precision%29))
  (|CallParentFunction NewStat)
  (bind _currentui (Class|BPIUserInterface|BPIGetCurrentUI(Message) (HUD|GetHUD (Game|GetPlayerController 0))))
  (Class|BPIUserInterface|BPIGetCurrentBossHealth(Message) _currentui (Variables|Default|GetCurrentStat))
  (if (<= (Variables|Default|GetCurrentStat) 0.0)
    (bind _assteel_player_character (Utilities|Casting|CastToSteelPlayerCharacter (Components|GetOwner)))
    (Default|MakeDeath _assteel_player_character)
    (CallFunction|MakeDeath)))

(fn MakeDeath
  (bind _asbp_main_game_mode (Utilities|Casting|CastToBP_Main_GameMode (Game|GetGameMode)))
  (Default|FinishGame _asbp_main_game_mode))