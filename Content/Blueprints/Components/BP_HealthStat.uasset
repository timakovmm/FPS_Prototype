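; BP_HealthStat is a health stat component that extends a parent stat class with HUD updates and armor gating.
; ChangeStat runs the parent logic, then passes the current value to the player 0 HUD's UI through Blueprint interface calls.
; TakeDamage forwards damage to the parent only when the owner's BP_ArmorStat component is exactly zero, so health takes no damage from that call while armor remains.
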(event EventBeginPlay
  (|CallParentFunction) ; This node is disabled and will not be called.\nDrag off pins to build functionality.
)

(event EventTick
  (params (DeltaSeconds :type Float%20%28single-precision%29)))

(fn ChangeStat
  (params (NewStat :type Float%20%28single-precision%29))
  (|CallParentFunction NewStat)
  (bind _currentui (Class|BPIUserInterface|BPIGetCurrentUI(Message) (HUD|GetHUD (Game|GetPlayerController 0))))
  (Class|BPIUserInterface|BPIGetCurrentHealth(Message) _currentui (Variables|Default|GetCurrentStat)))

(fn TakeDamage
  (params (DamageValue :type Float%20%28single-precision%29))
  (if (== (Variables|/Game/Blueprints/Components/BP_MainBioStat.BP_MainBioStat_C|GetCurrentStat (Actor|GetComponentbyClass (Components|GetOwner) "/Game/Blueprints/Components/BP_ArmorStat.BP_ArmorStat_C")) 0.0)
    (|CallParentFunction DamageValue)))