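; Component that spawns and manages the weapon carried by the Main_Character that owns it.
; On BeginPlay it spawns the configured CharacterWeapon class, stores the reference and attaches it to the character's skeletal mesh at the SocketWeapon socket.
; StartFire and StopFire forward to that weapon when it is valid, so firing logic stays in the weapon itself.
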(event EventBeginPlay
  (CallFunction|CreateWeapon))

(fn StartFire
  (if (Utilities|IsValid (Variables|Weapon|GetRefWeapon))
    (Default|StartFire (Variables|Weapon|GetRefWeapon))))

(fn StopFire
  (if (Utilities|IsValid (Variables|Weapon|GetRefWeapon))
    (Default|StopFire (Variables|Weapon|GetRefWeapon))))

(fn CreateWeapon
  (bind _characterweapon (Variables|Weapon|GetCharacterWeapon)
    (:then
      (bind _returnvalue (Game|SpawnActorfromClass _characterweapon (Math|Transform|MakeTransform "0, 0, 0") "AlwaysSpawn" 0 0))
      (Variables|Weapon|SetRefWeapon _returnvalue)
      (bind _asmain_character (Utilities|Casting|CastToMain_Character (Components|GetOwner)))
      (Transformation|AttachComponentToComponent (Variables|Weapon|GetRefWeapon) (Variables|/Game/Blueprints/Main_Character.Main_Character_C|GetSkeletalMesh _asmain_character) (Variables|Weapon|GetSocketWeapon) "KeepRelative" "KeepRelative" "KeepRelative" true))
    (:else)))