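; Player stat component that tracks clamped health and armor, filling both at BeginPlay and pushing changes to player 0's HUD through Blueprint interface messages.
; Damage hits armor first; if armor is at zero afterward, health also takes the full damage value, with no overflow math.
; Each hit halts armor regeneration and sets a delay timer, with a looping timer handling regeneration until armor is full.
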(event EventBeginPlay
  (Health|ChangeHealth (Variables|Health|GetMaxHealth))
  (Armor|ChangeArmor (Variables|Armor|GetMaxArmor)))

(fn AddHealth
  (params (AddHealth :type Float%20%28single-precision%29))
  (if (< (Variables|Health|GetCurrentHealth) (Variables|Health|GetMaxHealth))
    (Health|ChangeHealth (+ AddHealth (Variables|Health|GetCurrentHealth)))
    (return true)))

(fn DecreaseHealth
  (params (DamageValue :type Float%20%28single-precision%29))
  (Health|ChangeHealth (- (Variables|Health|GetCurrentHealth) DamageValue)))

(fn ChangeHealth
  (params (NewHealth :type Float%20%28single-precision%29))
  (if (!= NewHealth (Variables|Health|GetCurrentHealth))
    (Variables|Health|SetCurrentHealth (Math|Float|Clamp(Float) NewHealth 0.0 (Variables|Health|GetMaxHealth)))
    (bind _currentui (Class|BPIUserInterface|BPIGetCurrentUI(Message) (HUD|GetHUD (Game|GetPlayerController 0))))
    (Class|BPIUserInterface|BPIGetCurrentHealth(Message) _currentui (Variables|Health|GetCurrentHealth))))

(fn DecreaseArmor
  (params (DamageValue :type Float%20%28single-precision%29))
  (Utilities|Time|SetTimerbyEvent (EventDispatchers|CreateEvent :!event StartRegenerateArmor) (Variables|Armor|GetStartRegenerationDelay))
  (Armor|ChangeArmor (- (Variables|Armor|GetCurrentArmor) DamageValue))
  (Armor|StopRegenerateArmor))

(fn RegenerateArmor
  (Armor|ChangeArmor (+ (Variables|Armor|GetCurrentArmor) (Variables|Armor|GetRegenerationPower))))

(fn StartRegenerateArmor
  (bind _returnvalue (Utilities|Time|SetTimerbyEvent (EventDispatchers|CreateEvent :!event RegenerateArmor) (Variables|Armor|GetRegenerationRate) true))
  (Variables|Armor|SetRegenerationHandleTimer _returnvalue))

(fn StopRegenerateArmor
  (if (Utilities|Time|IsValidTimerHandle (Variables|Armor|GetRegenerationHandleTimer))
    (Utilities|Time|ClearandInvalidateTimerbyHandle (Variables|Armor|GetRegenerationHandleTimer))))

(fn ChangeArmor
  (params (NewArmor :type Float%20%28single-precision%29))
  (if (!= NewArmor (Variables|Armor|GetCurrentArmor))
    (Variables|Armor|SetCurrentArmor (Math|Float|Clamp(Float) NewArmor 0.0 (Variables|Armor|GetMaxArmor)))
    (bind _currentui (Class|BPIUserInterface|BPIGetCurrentUI(Message) (HUD|GetHUD (Game|GetPlayerController 0))))
    (Class|BPIUserInterface|BPIGetCurrentArmor(Message) _currentui (Variables|Armor|GetCurrentArmor))
    (if (== (Variables|Armor|GetCurrentArmor) (Variables|Armor|GetMaxArmor))
      (Armor|StopRegenerateArmor))))

(fn TakeDamage
  (params (DamageValue :type Float%20%28single-precision%29))
  (Armor|DecreaseArmor DamageValue)
  (if (== (Variables|Armor|GetCurrentArmor) 0.0)
    (Health|DecreaseHealth DamageValue)))