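; Rifle weapon Blueprint that extends a parent weapon class with automatic hitscan firing.
; StartFire runs Fire on a looping timer at FireRate, and StopFire clears that timer.
; Fire calls the parent, line-traces from player 0's camera along its view for FireDistance, and draws debug lines, including one from the muzzle socket.
; The hit result has no effect yet, and AddAmmo only calls the parent.
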(fn ConstructionScript
  (|CallParentFunction))

(fn Fire
  (bind _returnvalue (Game|GetPlayerController 0))
  (bind _firedistance (Variables|Default|GetFireDistance))
  (bind _playercameramanager (Variables|/Script/Engine.PlayerController|GetPlayerCameraManager _returnvalue))
  (bind _returnvalue_2 (Camera|GetCameraLocation _playercameramanager))
  (bind _returnvalue_3 (Camera|GetCameraRotation _playercameramanager))
  (bind _returnvalue_4 (Math|Vector|GetForwardVector _returnvalue_3))
  (bind _returnvalue_5 (* _returnvalue_4 _firedistance))
  (bind _returnvalue_6 (+ _returnvalue_2 _returnvalue_5))
  (|CallParentFunction)
  (bind (_outhit _returnvalue_7) (Collision|LineTraceByChannel _returnvalue_2 _returnvalue_6 "TraceTypeQuery1" false (Utilities|Array|MakeArray (Components|GetOwner)) "ForDuration"))
  (Rendering|Debug|DrawDebugLine (Transformation|GetSocketLocation (Variables|Default|GetWeaponBody) (Variables|Default|GetWeaponMuzzle)) _returnvalue_6 "(R=1.000000,G=0.000000,B=0.998857,A=1.000000)" 5.0 2.0)
  (if _returnvalue_7
    _))

(fn StartFire
  (bind _returnvalue (Utilities|Time|SetTimerbyFunctionName 0 "Fire" (Variables|Default|GetFireRate) true))
  (Variables|Default|SetFireHandle _returnvalue))

(fn StopFire
  (if (Utilities|Time|IsValidTimerHandle (Variables|Default|GetFireHandle))
    (Utilities|Time|ClearandInvalidateTimerbyHandle (Variables|Default|GetFireHandle))))

(fn AddAmmo
  (params (AddAmmo :type Integer))
  (|CallParentFunction AddAmmo))