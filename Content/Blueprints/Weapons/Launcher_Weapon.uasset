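; Launcher weapon Blueprint that spawns a WeaponBullet actor from the muzzle socket, aimed along the player camera's view.
; StartFire fires one shot if allowed, then blocks firing until a FireRate timer calls ResetFire; StopFire is empty.
; Fire calls the parent, then rotates the bullet toward a point FireDistance ahead of player 0's camera.
; Its debug-drawn visibility trace does not affect the aim, as the hit result is unused.
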(fn ConstructionScript
  (|CallParentFunction))

(fn Fire
  (bind _returnvalue (Game|GetPlayerController 0))
  (bind _playercameramanager (Variables|/Script/Engine.PlayerController|GetPlayerCameraManager _returnvalue))
  (|CallParentFunction)
  (LocalVariables|SetStartLocation (Transformation|GetSocketLocation (Variables|Default|GetWeaponBody) (Variables|Default|GetWeaponMuzzle)))
  (LocalVariables|SetEndLocation (+ (Camera|GetCameraLocation _playercameramanager) (* (Math|Vector|GetForwardVector (Camera|GetCameraRotation _playercameramanager)) (Variables|Default|GetFireDistance))))
  (Collision|LineTraceByChannel (LocalVariables|GetStartLocation) (LocalVariables|GetEndLocation) "TraceTypeQuery1" false (Utilities|Array|MakeArray (Components|GetOwner)) "ForDuration")
  (Game|SpawnActorfromClass "/Game/Blueprints/Weapons/WeaponBullet.WeaponBullet_C" (Math|Transform|MakeTransform (LocalVariables|GetStartLocation) (Math|Rotator|FindLookatRotation (LocalVariables|GetStartLocation) (LocalVariables|GetEndLocation))) "Undefined" 0 0))

(fn StartFire
  (if (Variables|Default|GetIsCanFire?)
    (Utilities|Time|SetTimerbyFunctionName 0 "ResetFire" (Variables|Default|GetFireRate))
    (CallFunction|Fire)
    (Variables|Default|SetIsCanFire? false)))

(fn StopFire)

(fn ResetFire
  (Variables|Default|SetIsCanFire? true))