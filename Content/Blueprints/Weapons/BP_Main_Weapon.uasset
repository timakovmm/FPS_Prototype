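; Main weapon Blueprint that handles firing state, magazine and reserve ammo, and reloading for the player character.
; Fire spends a round and plays the character's fire animation, auto-reloading when the magazine empties.
; StartReload cancels aiming, plays the reload animation and sets a timer for Reload, which refills from reserve.
; Clamped ammo setters update the HUD through interface messages when equipped; PauseFire is an empty stub.
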(fn ConstructionScript)

(fn Fire
  (bind _canfire_ (Fire|GetCanFire))
  (if _canfire_
    (Ammo|SubstractAmmo)
    (if (not (Variables|Reload|GetIsReloading?))
      (bind _asbp_main_character (Utilities|Casting|CastToBP_Main_Character (Game|GetPlayerCharacter 0)))
      (Default|FireAnimationStart _asbp_main_character (Variables|Fire|GetFireAnimation)))))

(fn StartFire
  (Variables|Fire|SetIsFiring? true))

(fn PauseFire
  (params (NewPause :type Boolean)))

(fn StopFire
  (Variables|Fire|SetIsFiring? false))

(fn GetCanFire
  (bind _output_get (Variables|Fire|SetCan%20Fire? (and (> (Variables|Ammo|GetCurrentAmmo) 0) (not (Variables|Reload|GetIsReloading?)))))
  (return _output_get))

(fn Reload
  (bind _leftammo (Variables|Ammo|GetLeftAmmo))
  (bind _ammodata (Variables|Ammo|GetAmmoData))
  (bind _currentammo (Variables|Ammo|GetCurrentAmmo))
  (bind _maxclipammo (Utilities|Struct|BreakStruct_Ammo _ammodata))
  (bind _returnvalue (- _maxclipammo _currentammo))
  (bind _output_get (LocalVariables|SetLocalAddAmmo (Math|Integer|SelectInt _leftammo _returnvalue (<= _leftammo _returnvalue))))
  (Ammo|ChangeCurrentAmmo (+ _output_get (Variables|Ammo|GetCurrentAmmo)))
  (Ammo|ChangeLeftAmmo (- (Variables|Ammo|GetLeftAmmo) (LocalVariables|GetLocalAddAmmo)))
  (Variables|Reload|SetIsReloading? false)
  (Development|PrintString "Reload!")
  (if (Variables|Fire|GetIsFiring?)
    (Fire|PauseFire false)
    (else
      (Fire|StopFire))))

(fn StartReload
  (if (not (Variables|Reload|GetIsReloading?))
    (if (and (> (Variables|Ammo|GetLeftAmmo) 0) (< (Variables|Ammo|GetCurrentAmmo) (.MaxClipAmmo (Utilities|Struct|BreakStruct_Ammo (Variables|Ammo|GetAmmoData)))))
      (bind _asbp_main_character (Utilities|Casting|CastToBP_Main_Character (Game|GetPlayerCharacter 0)))
      (bind _output_get (Variables|Default|SetCharacterRef _asbp_main_character))
      (if (Variables|/Game/Blueprints/Characters/BP_Main_Character.BP_Main_Character_C|GetIsAiming? _output_get)
        (Variables|/Game/Blueprints/Characters/BP_Main_Character.BP_Main_Character_C|SetIsAiming? (Variables|Default|GetCharacterRef) false))
      (bind _output_get_2 (Variables|Reload|SetIsReloading? true))
      (Fire|PauseFire _output_get_2)
      (Default|ReloadAnimationStart (Variables|Default|GetCharacterRef) (Variables|Reload|GetReloadAnimation))
      (Utilities|Time|SetTimerbyFunctionName 0 "Reload" (Variables|Reload|GetReloadTime)))))

(fn GetAmmoType
  (return (Variables|Ammo|GetAmmoType)))

(fn AddAmmo
  (params (AddAmmo :type Integer))
  (if (and (> AddAmmo 0) (< (Variables|Ammo|GetLeftAmmo) (.MaxAmmo (Utilities|Struct|BreakStruct_Ammo (Variables|Ammo|GetAmmoData)))))
    (Ammo|ChangeLeftAmmo (+ (Variables|Ammo|GetLeftAmmo) AddAmmo))
    (if (== (Variables|Ammo|GetCurrentAmmo) 0)
      (Reload|StartReload))))

(fn ChangeCurrentAmmo
  (params (ChangeCurrentAmmo :type Integer))
  (Variables|Ammo|SetCurrentAmmo (Math|Integer|Clamp(Integer) ChangeCurrentAmmo 0 (.MaxClipAmmo (Utilities|Struct|BreakStruct_Ammo (Variables|Ammo|GetAmmoData)))))
  (if (Variables|Default|GetIsEquipped?)
    (bind _currentui (Class|BPIUserInterface|BPIGetCurrentUI(Message) (HUD|GetHUD (Game|GetPlayerController 0))))
    (Class|BPIUserInterface|BPIGetCurrentAmmo(Message) _currentui (Variables|Ammo|GetCurrentAmmo))))

(fn ChangeLeftAmmo
  (params (ChangeLeftAmmo :type Integer))
  (Variables|Ammo|SetLeftAmmo (Math|Integer|Clamp(Integer) ChangeLeftAmmo 0 (.MaxAmmo (Utilities|Struct|BreakStruct_Ammo (Variables|Ammo|GetAmmoData)))))
  (if (Variables|Default|GetIsEquipped?)
    (bind _currentui (Class|BPIUserInterface|BPIGetCurrentUI(Message) (HUD|GetHUD (Game|GetPlayerController 0))))
    (Class|BPIUserInterface|BPIGetLeftAmmo(Message) _currentui (Variables|Ammo|GetLeftAmmo))))

(fn SubstractAmmo
  (Ammo|ChangeCurrentAmmo (- (Variables|Ammo|GetCurrentAmmo) 1))
  (if (== (Variables|Ammo|GetCurrentAmmo) 0)
    (if (> (Variables|Ammo|GetLeftAmmo) 0)
      (Reload|StartReload)
      (else
        (Fire|StopFire)))))