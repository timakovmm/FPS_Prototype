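; Behavior tree task that moves the AI pawn toward the player ahead of a bash, setting the BashType blackboard key.
; It resets BashType to 0 and runs AIMoveTo with a randomized timeout timer alongside.
; Reaching the player clears the timer and finishes successfully.
; SelectUltimateBashType, apparently the timer callback, switches BashType to 1, stops movement and finishes successfully.
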(event EventReceiveExecuteAI
  (params (OwnerController :type AI%20Controller%20Object%20Reference) (ControlledPawn :type Pawn%20Object%20Reference))
  (Variables|Default|SetAIControllerRef OwnerController)
  (Class|BTFunctionLibrary|SetBlackboardValueasEnum (Variables|Default|GetBashType))
  (bind _returnvalue (Utilities|Time|SetTimerbyEvent (EventDispatchers|CreateEvent :!event SelectUltimateBashType) (Math|Random|RandomFloatinRange 5.0 8.0)))
  (Variables|Default|SetTimerHandler _returnvalue)
  (AI|AIMoveTo ControlledPawn "0, 0, 0" (Game|GetPlayerCharacter 0) 4e+02 false
    (:OnSuccess
      (Utilities|Time|ClearandInvalidateTimerbyHandle (Variables|Default|GetTimerHandler))
      (AI|BehaviorTree|FinishExecute true))))

(fn SelectUltimateBashType
  (Class|BTFunctionLibrary|SetBlackboardValueasEnum (Variables|Default|GetBashType) 1)
  (AI|Navigation|StopMovement (Variables|Default|GetAIControllerRef))
  (AI|BehaviorTree|FinishExecute true))