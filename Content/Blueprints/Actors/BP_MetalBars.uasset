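; BP_MetalBars is a boss fight trigger that moves a set of metal bars when the player character enters its box.
; The first overlap by BP_Main_Character disables the box collision, so it fires once, and plays the boss fight sound from an offset.
; A timeline slides the mesh vertically between two relative positions.
; When it finishes, it calls BeginAI on the BP_AI_BossController of BossRef, if that reference is valid.
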(event OnComponentBeginOverlap(Box)
  (params (OverlappedComponent :type Primitive%20Component%20Object%20Reference) (OtherActor :type Actor%20Object%20Reference) (OtherComp :type Primitive%20Component%20Object%20Reference) (OtherBodyIndex :type Integer) (bFromSweep :type Boolean) (SweepResult :type Hit%20Result%20Structure%20%28by%20ref%29))
  (bind _bossref (Variables|Default|GetBossRef))
  (Utilities|Casting|CastToBP_Main_Character OtherActor)
  (Collision|SetCollisionEnabled (Variables|Default|GetBox) "NoCollision")
  (Audio|PlaySoundatLocation "/Game/Blueprints/Audio/AF_BossFight.AF_BossFight" "0, 0, 0" "0, 0, 0" 0.1 1.0 3.4 0 0 0)
  (bind _lerp (Timeline|MetalBars Play)
    (:Update
      (Transformation|SetRelativeLocation (Variables|Default|GetStaticMesh) (Math|Vector|Lerp(Vector) "0,-150.000000,95.000000" "0,-150.000000,-175.000000" _lerp) false false))
    (:Finished
      (Utilities|IsValid _bossref
        (:Is%20Valid
          (bind _asbp_ai_boss_controller (Utilities|Casting|CastToBP_AI_BossController (Pawn|GetController _bossref)))
          (Default|BeginAI _asbp_ai_boss_controller))))))

(fn ConstructionScript)